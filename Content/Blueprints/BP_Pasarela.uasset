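; BP_Pasarela is a walkway that starts hidden without collision and can be switched on and off.
; Its construction script applies the CustomMesh and MeshMat variables to the static mesh, then hides it and disables collision.
; Each ActivarAsociado event alternates through a FlipFlop between showing the mesh with query and physics collision and hiding it with no collision.
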(event `/Game/Blueprints/I_Asociado.Activar Asociado`
  (bind _staticmesh (`self.StaticMesh`))
  (`/Engine/EditorBlueprintResources/StandardMacros.FlipFlop`
    (:`A`
      (`SceneComponent.SetVisibility` _staticmesh true false)
      (`PrimitiveComponent.SetCollisionEnabled` _staticmesh "QueryAndPhysics"))
    (:`B`
      (`SceneComponent.SetVisibility` _staticmesh false false)
      (`PrimitiveComponent.SetCollisionEnabled` _staticmesh "NoCollision"))))

(fn `UserConstructionScript`
  (bind _staticmesh (`self.StaticMesh`))
  (`StaticMeshComponent.SetStaticMesh` (`self.StaticMesh`) (`self.CustomMesh`))
  (`SceneComponent.SetVisibility` _staticmesh false false)
  (`PrimitiveComponent.SetCollisionEnabled` _staticmesh "NoCollision")
  (`PrimitiveComponent.SetMaterial` _staticmesh 0 (`self.MeshMat`)))