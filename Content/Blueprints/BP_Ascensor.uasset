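; BP_Ascensor is an elevator that moves between its placed location and FinalPos, starting on BeginPlay or through ActivarAsociado.
; Ida and Vuelta timelines lerp the actor location, both rate-scaled by TiempoIda.
; EnEjecucion blocks re-triggering and FinUp selects direction, while UpDown chains an automatic return and Loop repeats the cycle.
; The construction script captures InitPos and copies the linked PulsadorAsociado's decal and help text, hiding the icon without one.
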(event `self.ReceiveBeginPlay`
  ;[1 1 1] Si el ascensor empieza activado
  (if (`self.StartActivado`)
    (`/Game/Blueprints/I_Asociado.Activar Asociado`)))

(event `/Game/Blueprints/I_Asociado.Activar Asociado`
  (if (not (`self.EnEjecucion`))
    (set `self.EnEjecucion` true)
    (if (not (`self.FinUp`))
      (bind (_direction _track_0) (`Timeline|Ida` :!via `PlayFromStart` :!label _label)
        (:`Update`
          (`self.K2_SetActorLocation` (`KismetMathLibrary.VLerp` (`self.InitPos`) (`self.FinalPos`) _track_0)))
        (:`Finished`
          (set `self.FinUp` true)
          (if (`self.UpDown`)
            (bind (_direction_2 _track_0_2) (`Timeline|Vuelta` :!via `PlayFromStart` :!label _label_2)
              (:`Update`
                (`self.K2_SetActorLocation` (`KismetMathLibrary.VLerp` (`self.FinalPos`) (`self.InitPos`) _track_0_2)))
              (:`Finished`
                (set `self.FinUp` false)
                (if (`self.Loop`)
                  (goto _label :!via `PlayFromStart`)
                  (else
                    (set `self.EnEjecucion` false)))))
            (else
              (set `self.EnEjecucion` false)))))
      (else
        (goto _label_2 :!via `PlayFromStart`)))))

(fn `UserConstructionScript`
  (bind _pulsadorasociado (`self.PulsadorAsociado`))
  (bind _icono (`self.Icono`))
  (bind _returnvalue (/ 1.0 (`self.TiempoIda`)))
  (set `self.InitPos` (`self.K2_GetActorLocation`))
  (`TimelineComponent.SetPlayRate` (`self.Ida`) _returnvalue)
  (`TimelineComponent.SetPlayRate` (`self.Vuelta`) _returnvalue)
  (if (`KismetSystemLibrary.IsValid` _pulsadorasociado)
    (bind _icono_2 (`/Game/Blueprints/BP_Pulsador.Icono` _pulsadorasociado)
      (:`then`
        (`DecalComponent.SetDecalMaterial` _icono (`DecalComponent.GetDecalMaterial` _icono_2))
        (`TextRenderComponent.K2_SetText` (`self.TextoPulsador`) (`/Game/Blueprints/BP_Pulsador.TextoAyuda` _pulsadorasociado)))
      (:`else`))
    (else
      (`SceneComponent.SetVisibility` _icono false false))))