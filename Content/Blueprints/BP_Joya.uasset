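; BP_Joya is a gem pickup that rewards the player with extra time and adds to the gem count.
; When a BP_Peon overlaps its capsule, it writes both values directly into that pawn's MyGui.
; It then plays the diamond sound, spawns the N_Diamond Niagara effect at the capsule's location and destroys itself.
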(event `self.Capsule.OnComponentBeginOverlap`
  (params (OverlappedComponent :type "PrimitiveComponent Object Reference") (OtherActor :type "Actor Object Reference") (OtherComp :type "PrimitiveComponent Object Reference") (OtherBodyIndex :type Integer) (bFromSweep :type Boolean) (SweepResult :type "HitResult Structure (by ref)"))
  (bind (_asbp_peon _bsuccess) (cast `/Game/Blueprints/BP_Peon` OtherActor :!pure true))
  (bind _mygui (`/Game/Blueprints/BP_Peon.MyGui` _asbp_peon))
  (bind _returnvalue (`SceneComponent.K2_GetComponentLocation` (`self.Capsule`)))
  (if _bsuccess
    (set `/Game/Blueprints/UI_Datos.ExtraTime` (+ (`/Game/Blueprints/UI_Datos.ExtraTime` _mygui) 10.0) _mygui)
    (bind _result (`/Engine/EditorBlueprintResources/StandardMacros.IncrementInt` (`/Game/Blueprints/UI_Datos.Joyas` _mygui))
      (:`  `
        (set `/Game/Blueprints/UI_Datos.Joyas` _result _mygui)
        (`GameplayStatics.PlaySoundAtLocation` "/Game/Sonidos/Audio_Diamante.Audio_Diamante" _returnvalue (struct) 1.0 1.0 0.0 null null null null)
        (`NiagaraFunctionLibrary.SpawnSystemAtLocation` "/Game/Niagara/N_Diamond.N_Diamond" _returnvalue)
        (`self.K2_DestroyActor`)))))

(fn `UserConstructionScript`)