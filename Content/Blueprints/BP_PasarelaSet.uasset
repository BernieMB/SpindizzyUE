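; BP_PasarelaSet is a walkway actor that can be switched on or off, toggling both its visibility and collision.
; The construction script applies a configurable mesh and material and sets the initial state from ActivadaDefault, printing a leftover "Hello" when active.
; BeginPlay reapplies the active state if enabled by default.
; SetAsociado(Activar) waits a configurable delay, then shows it with collision or hides it without.
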(event `self.ReceiveBeginPlay`
  (bind _staticmesh (`self.StaticMesh`))
  (if (`self.ActivadaDefault`)
    (`SceneComponent.SetVisibility` _staticmesh true false)
    (`PrimitiveComponent.SetCollisionEnabled` _staticmesh "QueryAndPhysics")))

(event `/Game/Blueprints/I_SetAsociado.SetAsociado`
  (params (Activar :type Boolean))
  (bind _staticmesh (`self.StaticMesh`))
  (`KismetSystemLibrary.Delay` (`self.Delay`))
  (if Activar
    (`SceneComponent.SetVisibility` _staticmesh true false)
    (`PrimitiveComponent.SetCollisionEnabled` _staticmesh "QueryAndPhysics")
    (else
      (`SceneComponent.SetVisibility` _staticmesh false false)
      (`PrimitiveComponent.SetCollisionEnabled` _staticmesh "NoCollision"))))

(fn `UserConstructionScript`
  (bind _activadadefault (`self.ActivadaDefault`))
  (bind _staticmesh (`self.StaticMesh`))
  (`StaticMeshComponent.SetStaticMesh` (`self.StaticMesh`) (`self.CustomMesh`))
  (`SceneComponent.SetVisibility` _staticmesh _activadadefault true)
  (`PrimitiveComponent.SetMaterial` _staticmesh 0 (`self.MeshMat`))
  (if _activadadefault
    (`PrimitiveComponent.SetCollisionEnabled` _staticmesh "QueryAndPhysics")
    (`KismetSystemLibrary.PrintString` "Hello")
    (else
      (`PrimitiveComponent.SetCollisionEnabled` _staticmesh "NoCollision"))))