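; BP_Enemy is an enemy whose physics-driven Cone chases the player's BP_Peon while it is inside the ZonaActiva box, sized by ZonaAcceso.
; Overlap begin checks the component's "Player" tag to store the target and activate; overlap end checks the actor's tag to deactivate and zero Cone velocity.
; While active, Tick applies horizontal velocity-change impulses toward the target's SphereCollision, scaled by EnemyVelocity and delta time.
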(event `self.ReceiveBeginPlay`
  (`BoxComponent.SetBoxExtent` (`self.ZonaActiva`) (`self.ZonaAcceso`) true))

(event `self.ReceiveTick`
  (params (DeltaSeconds :type "Float (single-precision)"))
  (bind (_returnvalue_x _returnvalue_y) (`KismetMathLibrary.BreakVector` (* DeltaSeconds (`self.EnemyVelocity`) (`KismetMathLibrary.Normal` (- (`SceneComponent.K2_GetComponentLocation` (`/Game/Blueprints/BP_Peon.SphereCollision` (`self.OtherActor`))) (`SceneComponent.K2_GetComponentLocation` (`self.Cone`)))))))
  (if (`self.Activado`)
    (`PrimitiveComponent.AddImpulse` (`self.Cone`) (`KismetMathLibrary.MakeVector` _returnvalue_x _returnvalue_y) "None" true)))

(event `self.ZonaActiva.OnComponentBeginOverlap`
  (params (OverlappedComponent :type "PrimitiveComponent Object Reference") (OtherActor :type "Actor Object Reference") (OtherComp :type "PrimitiveComponent Object Reference") (OtherBodyIndex :type Integer) (bFromSweep :type Boolean) (SweepResult :type "HitResult Structure (by ref)"))
  (if (`ActorComponent.ComponentHasTag` OtherComp "Player")
    (set `self.OtherActor` (cast `/Game/Blueprints/BP_Peon` OtherActor :!pure true))
    (set `self.Activado` true)))

(event `self.ZonaActiva.OnComponentEndOverlap`
  (params (OverlappedComponent :type "PrimitiveComponent Object Reference") (OtherActor :type "Actor Object Reference") (OtherComp :type "PrimitiveComponent Object Reference") (OtherBodyIndex :type Integer))
  (if (`self.ActorHasTag` OtherActor "Player")
    (set `self.Activado` false)
    (`PrimitiveComponent.SetPhysicsLinearVelocity` (`self.Cone`) (0.0 0.0 0.0) false "None")))

(fn `UserConstructionScript`
  (`BoxComponent.SetBoxExtent` (`self.ZonaActiva`) (`self.ZonaAcceso`) true))