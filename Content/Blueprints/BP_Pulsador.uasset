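; BP_Pulsador is a trigger button that signals an associated actor when a Player-tagged actor overlaps its box.
; While Activado, it sends either an activate message or a set-state message through Asociado, then plays an elevator sound.
; An optional single-use mode gates this through a DoOnce, which ResetTrigger re-arms.
; The construction script applies help text and trigger size, and configures the icon decal's material, scale and optional flip.
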(event `self.BoxCollision.OnComponentBeginOverlap`
  (params (OverlappedComponent :type "PrimitiveComponent Object Reference") (OtherActor :type "Actor Object Reference") (OtherComp :type "PrimitiveComponent Object Reference") (OtherBodyIndex :type Integer) (bFromSweep :type Boolean) (SweepResult :type "HitResult Structure (by ref)"))
  (bind _asociado (`self.Asociado`))
  (if (`self.ActorHasTag` OtherActor "Player")
    (if (`self.Activado`)
      (if (`self.UnUso`)
        (`/Engine/EditorBlueprintResources/StandardMacros.DoOnce` false :!label _label
          (:`Completed`
            _)))
      (if (not (`self.SetAsociado`))
        (message `/Game/Blueprints/I_Asociado.Activar Asociado` _asociado)
        (else
          (message `/Game/Blueprints/I_SetAsociado.SetAsociado` _asociado (`self.ActivarAsociado`))))
      (`GameplayStatics.PlaySoundAtLocation` "/Game/Sonidos/Audio_Ascensor.Audio_Ascensor" (`SceneComponent.K2_GetComponentLocation` (`self.DefaultSceneRoot`)) (struct) 1.0 1.0 0.0 null null null null))))

(event `ResetTrigger`
  (goto _label :!via `Reset`))

(fn `UserConstructionScript`
  (bind (_sizetrigger_x _sizetrigger_y _sizetrigger_z) (`KismetMathLibrary.BreakVector` (`self.SizeTrigger`)))
  (bind _icono (`self.Icono`))
  (`TextRenderComponent.K2_SetText` (`self.Text`) (`self.TextoAyuda`))
  (`BoxComponent.SetBoxExtent` (`self.BoxCollision`) (`self.SizeTrigger`) true)
  (`SceneComponent.SetRelativeScale3D` _icono (`KismetMathLibrary.MakeVector` _sizetrigger_z _sizetrigger_y _sizetrigger_x))
  (`DecalComponent.SetDecalMaterial` _icono (`self.IconoMat`))
  (if (`self.Inverted`)
    (`SceneComponent.K2_AddRelativeRotation` (`self.Icono`) (struct :`Roll` 180.0) false false)))